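; Manager for a timed bottle-shaking minigame that builds soda pressure from Joy-Con motion.
; Enter, guarded by a DoOnce, zeroes timer and pressure and opens a Tick gate.
; While open, the gate adds absolute gyro pitch velocity to SodaPower every frame and rumbles the Joy-Con.
; Passing TimeLimit closes the gate and re-arms Enter; gyro, pressure and remaining time print on screen as debug text.
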(event `Key|Enter`
  (params (Key :type "Key Structure"))
  ;[1 1 1] 瓶振りの開始
  (:`Pressed`
    (`/Engine/EditorBlueprintResources/StandardMacros.DoOnce` false :!label _label
      (:`Completed`
        (`self.StartShaking`)
        (set `self.Timer` 0.0)
        (set `self.SodaPower` 0.0)))))

(event `ResetTimer`
  ;[1 1 1] 瓶振りの開始
  (goto _label :!via `Reset`))

(event `self.ReceiveTick`
  (params (DeltaSeconds :type "Float (single-precision)"))
  (bind (_success _gyroscope) (`JoyConDriverFunctionLibrary.GetJoyConGyroscope` 0))
  (bind (_angularvelocity_roll _angularvelocity_pitch) (`KismetMathLibrary.BreakRotator` (`self.AngularVelocity`)))
  (bind _returnvalue (`KismetMathLibrary.MakeRotator` (* (.x _gyroscope) -1.0) (* (.y _gyroscope) -1.0) (.z _gyroscope)))
  (set `self.Delta Seconds` DeltaSeconds)
  (`|ExecutionSequence`
    (:`then_0`
      ;[1 1 1] 角速度の計測
      (if _success
        (set `self.AngularVelocity` _returnvalue)
        (`KismetSystemLibrary.PrintString` (`KismetStringLibrary.Concat_StrStr` "Angular velocity is: " (`KismetStringLibrary.Conv_RotatorToString` _returnvalue)) true false (struct :`R` 0.351533 :`G` 0.982251 :`B` 0.059512 :`A` 1.0) (`self.Delta Seconds`))))
    (:`then_1`
      ;[1 1 1] 瓶の圧力を上げる処理
      (`/Engine/EditorBlueprintResources/StandardMacros.Gate` true :!label _label_2
        (:`Exit`
          (`|ExecutionSequence`
            (:`then_0`
              ;;[1 1 1] 瓶の圧力の加算
              (set `self.SodaPower` (+ (`self.SodaPower`) (`KismetMathLibrary.Abs` _angularvelocity_pitch)))
              ;;[1 1 1] 時間の計測
              (bind _output_get (set `self.Timer` (+ (`self.Timer`) (`self.Delta Seconds`))))
              ;;[1 1 1] タイマーのリセットと圧力加算の停止
              (if (> _output_get (`self.TimeLimit`))
                (`self.StopShaking`)
                (`self.ResetTimer`)))
            (:`then_1`
              (`JoyConDriverFunctionLibrary.SetJoyConRumble` 0 200.0 600.0 0.6 1))))))
    (:`then_2`
      ;[1 1 1] 瓶の圧力とタイマーの表示
      (`KismetSystemLibrary.PrintString` (`KismetStringLibrary.Concat_StrStr` "SodaPower Is: " (`KismetStringLibrary.Conv_DoubleToString` (`self.SodaPower`))) true false (struct :`G` 0.98315 :`B` 1.0 :`A` 1.0) (`self.Delta Seconds`))
      (`KismetSystemLibrary.PrintString` (`KismetStringLibrary.Concat_StrStr` "Remain Time Is: " (`KismetStringLibrary.Conv_DoubleToString` (- (`self.TimeLimit`) (`self.Timer`)))) true false (struct :`R` 0.945494 :`B` 1.0 :`A` 1.0) (`self.Delta Seconds`)))))

(event `StartShaking`
  ;[1 1 1] 瓶の圧力を上げる処理
  (goto _label_2 :!via `Open`))

(event `StopShaking`
  ;[1 1 1] 瓶の圧力を上げる処理
  (goto _label_2 :!via `Close`))

(fn `UserConstructionScript`)