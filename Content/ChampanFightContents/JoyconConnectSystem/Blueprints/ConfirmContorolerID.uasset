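; Joy-Con test Blueprint for up to four controllers that either mirrors their rotation or rumbles them for ID confirmation, depending on GameState.
; BeginPlay and the R key re-center all four and set portrait grip.
; Each Tick, SynthRotation applies axis-corrected orientation to Root1–4 and stores accelerometer and gyroscope readings.
; Confirm mode sets a RumbleState label and rumbles each controller; its trailing Delay does not stagger the loop.
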(event `self.ReceiveBeginPlay`
  ;[1 1 1] Joyconのリセット
  (for _index (range 4) :!label _label
    (`JoyConDriverFunctionLibrary.ReCenterJoyCon` _index)
    (`JoyConDriverFunctionLibrary.SetJoyConGripMode` _index "Portrait"))
  (`KismetSystemLibrary.PrintString` "Joycon Re Centerd"))

(event `Key|R` :consume false
  (params (Key :type "Key Structure"))
  ;[1 1 1] Joyconのリセット
  (:`Pressed`
    (goto _label)))

(event `self.ReceiveTick`
  (params (DeltaSeconds :type "Float (single-precision)"))
  (set `self.Delta Seconds` DeltaSeconds)
  (switch `string` (`self.GameState`)
    (:`SynthRotation`
      (for _index (range 4)
        (set `self.ControllerID` _index)
        (`self.SynthRotation`)))
    (:`ConfirmControllerID`
      (for _index_2 (range 4)
        (set `self.ControllerID` _index_2)
        (switch `int` (`self.ControllerID`)
          (:`0`
            (set `self.RumbleState` "Contoroller1"))
          (:`1`
            (set `self.RumbleState` "Contoroller2"))
          (:`2`
            (set `self.RumbleState` "Contoroller3"))
          (:`3`
            (set `self.RumbleState` "Contoroller4")))
        (`JoyConDriverFunctionLibrary.SetJoyConRumble` (`self.ControllerID`) 180.0 360.0 0.0 5)
        (`KismetSystemLibrary.Delay` 6.0))
      (set `self.RumbleState` "null"))))

(fn `SynthRotation`
  (bind (_success _accelerometer) (`JoyConDriverFunctionLibrary.GetJoyConAccelerometer` (`self.ControllerID`)))
  (bind (_success_2 _vector) (`JoyConDriverFunctionLibrary.GetJoyConVector` (`self.ControllerID`)))
  (bind (_success_3 _gyroscope) (`JoyConDriverFunctionLibrary.GetJoyConGyroscope` (`self.ControllerID`)))
  (bind _returnvalue (`KismetMathLibrary.MakeVector` (* (.x _accelerometer) -1.0) (* (.y _accelerometer) -1.0) (.z _accelerometer)))
  (bind _returnvalue_2 (`KismetMathLibrary.MakeRotator` (* (.x _gyroscope) -1.0) (* (.y _gyroscope) -1.0) (.z _gyroscope)))
  (switch `int` (`self.ControllerID`)
    (:`0`
      (set `self.RotateTarget` (`self.root1`)))
    (:`1`
      (set `self.RotateTarget` (`self.root2`)))
    (:`2`
      (set `self.RotateTarget` (`self.root3`)))
    (:`3`
      (set `self.RotateTarget` (`self.root4`))))
  (`|ExecutionSequence`
    (:`then_0`
      ;[1 1 1] 姿勢
      (if _success
        (set `self.Posture` _returnvalue)
        (`KismetSystemLibrary.PrintString` (`KismetStringLibrary.Concat_StrStr` "Posture is: " (`KismetStringLibrary.Conv_VectorToString` _returnvalue)) false false (struct :`R` 0.964686 :`G` 0.571125 :`B` 0.016807 :`A` 1.0) (`self.Delta Seconds`))))
    (:`then_1`
      ;[1 1 1] 角速度
      (if _success_3
        (set `self.AngularVelocity` _returnvalue_2)
        (`KismetSystemLibrary.PrintString` (`KismetStringLibrary.Concat_StrStr` "Angular velocity is: " (`KismetStringLibrary.Conv_RotatorToString` _returnvalue_2)) false false (struct :`R` 0.351533 :`G` 0.982251 :`B` 0.059512 :`A` 1.0) (`self.Delta Seconds`))))
    (:`then_2`
      ;[1 1 1] 角度
      (if _success_2
        (set `self.Angle` (`KismetMathLibrary.MakeRotator` (* (.roll _vector) -1.0) (* (.pitch _vector) -1.0) (.yaw _vector)))
        (`KismetSystemLibrary.PrintString` (`KismetStringLibrary.Concat_StrStr` "Angle is: " (`KismetStringLibrary.Conv_RotatorToString` (struct))) false false (struct :`R` 0.351532 :`G` 0.445201 :`B` 0.973445 :`A` 1.0) (`self.Delta Seconds`))))
    (:`then_3`
      ;[1 1 1] 座標の同期
      (`SceneComponent.K2_SetRelativeRotation` (`self.RotateTarget`) (`self.Angle`) false false))))

(fn `UserConstructionScript`)