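; Player 1's explodable bottle in the Joy-Con connect system, which damages itself when that player's break flag is set.
; On BeginPlay it caches the BP_ConfirmControllerID_2 actor found by the ConfirmContorollerID tag.
; Tick polls that actor's 1PBroke flag and applies self-damage once, while the Enter key applies the same damage directly.
; The graph holds no explosion logic of its own, only the damage trigger.
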(event `self.ReceiveBeginPlay`
  (bind _outactors (`GameplayStatics.GetAllActorsWithTag` "ConfirmContorollerID"))
  (for _array_element _outactors
    (bind _asbp_confirm_controller_id_2 (cast `/Game/ChampanFightContents/JoyconConnectSystem/Blueprints/BP_ConfirmControllerID_2` _array_element))
    (set `self.Confirm Controller ID Reference` _asbp_confirm_controller_id_2)))

(event `self.ReceiveTick`
  (params (DeltaSeconds :type "Float (single-precision)"))
  (if (`/Game/ChampanFightContents/JoyconConnectSystem/Blueprints/BP_ConfirmControllerID_2.1PBroke` (`self.Confirm Controller ID Reference`))
    (`/Engine/EditorBlueprintResources/StandardMacros.DoOnce` false
      (:`Completed`
        (`GameplayStatics.ApplyDamage` self 100.0)))))

(event `Key|Enter` :consume false
  (params (Key :type "Key Structure"))
  (:`Pressed`
    (`GameplayStatics.ApplyDamage` self 100.0)))

(fn `UserConstructionScript`
  (`parent.UserConstructionScript`))