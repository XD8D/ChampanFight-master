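; Two-player Joy-Con shaking game actor that charges soda bottles until one exceeds its limit and breaks.
; Tick adds each controller's gyro pitch rate above a threshold to that player's soda power, driving sine-based bottle bobbing and rumble strength.
; Exceeding the max sets that player's broke flag and stops the updates, resetting bottle positions.
; Win events spawn Niagara splashes at each player's particle root, and the R key recenters both Joy-Cons.
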(event `Key|R` :consume false
  (params (Key :type "Key Structure"))
  ;[1 1 1] Joyconのリセット
  (:`Pressed`
    (for _index (range 2)
      (`JoyConDriverFunctionLibrary.ReCenterJoyCon` _index)
      (`JoyConDriverFunctionLibrary.SetJoyConGripMode` _index "Portrait"))
    (`KismetSystemLibrary.PrintString` "Joycon Re Centerd")))

(event `1PWin`
  ;[1 1 1] 水しぶきを出す処理
  (`NiagaraFunctionLibrary.SpawnSystemAtLocation` "/Game/ChampanFightContents/KERO/FX/NewNiagaraSystem.NewNiagaraSystem" (`SceneComponent.K2_GetComponentLocation` (`self.1PParticleRoot`))))

(event `2PWin`
  ;[1 1 1] 水しぶきを出す処理
  (`NiagaraFunctionLibrary.SpawnSystemAtLocation` "/Game/ChampanFightContents/KERO/FX/NewNiagaraSystem.NewNiagaraSystem" (`SceneComponent.K2_GetComponentLocation` (`self.2PParticleRoot`))))

(event `self.ReceiveTick`
  (params (DeltaSeconds :type "Float (single-precision)"))
  ;[1 1 1] ゲームが終了したときは実行しない
  (set `self.Delta Seconds` DeltaSeconds)
  (if (== (`self.Checker_vibration`) 0)
    (`self.GetAngularVelocity`)
    (`self.vibration`)
    (`KismetSystemLibrary.PrintString` (`KismetStringLibrary.Conv_DoubleToString` (`self.SodaPower0`)) false false)
    (`/Engine/EditorBlueprintResources/StandardMacros.DoOnce` false
      (:`Completed`
        (`self.Get_maxsoda`)))
    (else
      (`SceneComponent.K2_SetRelativeLocation` (`self.root1`) (60.0 0.0 0.0) false false)
      (`SceneComponent.K2_SetRelativeLocation` (`self.root2`) (-60.0 0.0 0.0) false false))))

(fn `GetAngularVelocity`
  (bind (_success _gyroscope) (`JoyConDriverFunctionLibrary.GetJoyConGyroscope` (`self.ControllerID`)))
  (bind _returnvalue (`KismetMathLibrary.Abs` (`|GetArrayItem` (`self.YAngularVelocity `) 1)))
  (bind _returnvalue_2 (`KismetMathLibrary.Abs` (`|GetArrayItem` (`self.YAngularVelocity `))))
  (bind (_returnvalue_roll _returnvalue_pitch) (`KismetMathLibrary.BreakRotator` (`KismetMathLibrary.MakeRotator` (* (.x _gyroscope) -1.0) (* (.y _gyroscope) -1.0) (.z _gyroscope))))
  (for _index (range 2)
    (set `self.ControllerID` _index)
    ;[1 1 1] 角速度の計測+累計
    (if _success
      (`KismetArrayLibrary.Array_Insert` (`self.YAngularVelocity `) _returnvalue_pitch (`self.ControllerID`))))
  ;[1 1 1] Y軸速度が一定以上の値の時のみ、値を計測する。
  (`|ExecutionSequence`
    (:`then_0`
      (if (> _returnvalue_2 0.1)
        (set `self.SodaPower0` (+ (`self.SodaPower0`) (* _returnvalue_2 (`self.SodaPowerMultiply`))))))
    (:`then_1`
      (if (> _returnvalue 0.1)
        (set `self.SodaPower1` (+ (`self.SodaPower1`) (* _returnvalue (`self.SodaPowerMultiply`))))))))

(fn `UserConstructionScript`)

(fn `vibration`
  (bind _sodapower1 (`self.SodaPower1`))
  (bind _sodapower0 (`self.SodaPower0`))
  ;[1 1 1] 1P側の振動と瓶の振動
  (`SceneComponent.K2_SetRelativeLocation` (`self.root1`) (`KismetMathLibrary.MakeVector` 60.0 0.0 (* (`KismetMathLibrary.Sin` _sodapower0) 20.0)) false false)
  (`JoyConDriverFunctionLibrary.SetJoyConRumble` 0 200.0 600.0 (`KismetMathLibrary.FClamp` (* _sodapower0 0.0002) 0.1) 2)
  ;[1 1 1] 2Pの振動と瓶の振動
  (`SceneComponent.K2_SetRelativeLocation` (`self.root2`) (`KismetMathLibrary.MakeVector` -60.0 0.0 (* (`KismetMathLibrary.Sin` _sodapower1) 20.0)) false false)
  (`JoyConDriverFunctionLibrary.SetJoyConRumble` 1 200.0 600.0 (`KismetMathLibrary.FClamp` (* _sodapower1 0.0002) 0.01) 2)
  ;[1 1 1] ソーダパワーが限界値を超えたら瓶が割れる
  (`|ExecutionSequence`
    (:`then_0`
      (if (> (`self.SodaPower0`) (`self.SodaMaxPower`))
        (set `self.Checker_vibration` 1)
        (set `self.1PBroke` true)))
    (:`then_1`
      (if (> (`self.SodaPower1`) (`self.SodaMaxPower`))
        (set `self.Checker_vibration` 2)
        (set `self.2PBroke` true)))
    (:`then_2`
      (return))))