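; BP_Joycon is a prototype actor that mirrors the motion of the first Joy-Con controller onto its Joycon component.
; It recenters the controller in portrait grip on BeginPlay or when R is pressed.
; Each tick it stores axis-flipped accelerometer, gyroscope and orientation readings as posture, angular velocity and angle.
; The angle then sets the component's relative rotation, and its yaw and pitch, scaled by Sensitivity, drive its relative position.
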(event `self.ReceiveBeginPlay`
  ;[1 1 1] Joyconのリセット
  (`JoyConDriverFunctionLibrary.ReCenterJoyCon` 0 :!label _label)
  (`JoyConDriverFunctionLibrary.SetJoyConGripMode` 0 "Portrait")
  (`KismetSystemLibrary.PrintString` "Joycon Re Centerd"))

(event `Key|R` :consume false
  (params (Key :type "Key Structure"))
  ;[1 1 1] Joyconのリセット
  (:`Pressed`
    (goto _label)))

(event `self.ReceiveTick`
  (params (DeltaSeconds :type "Float (single-precision)"))
  (bind (_success _accelerometer) (`JoyConDriverFunctionLibrary.GetJoyConAccelerometer` 0))
  (bind (_success_2 _vector) (`JoyConDriverFunctionLibrary.GetJoyConVector` 0))
  (bind (_success_3 _gyroscope) (`JoyConDriverFunctionLibrary.GetJoyConGyroscope` 0))
  (bind _angle (`self.Angle`))
  (bind _returnvalue (`KismetMathLibrary.MakeVector` (* (.x _accelerometer) -1.0) (* (.y _accelerometer) -1.0) (.z _accelerometer)))
  (bind _returnvalue_2 (`KismetMathLibrary.MakeRotator` (* (.x _gyroscope) -1.0) (* (.y _gyroscope) -1.0) (.z _gyroscope)))
  (set `self.Delta Seconds` DeltaSeconds)
  (`|ExecutionSequence`
    (:`then_0`
      ;[1 1 1] 姿勢
      (if _success
        (set `self.Posture` _returnvalue)
        (`KismetSystemLibrary.PrintString` (`KismetStringLibrary.Concat_StrStr` "Posture is: " (`KismetStringLibrary.Conv_VectorToString` _returnvalue)) false false (struct :`R` 0.964686 :`G` 0.571125 :`B` 0.016807 :`A` 1.0) (`self.Delta Seconds`))))
    (:`then_1`
      ;[1 1 1] 角速度
      (if _success_3
        (set `self.AngularVelocity` _returnvalue_2)
        (`KismetSystemLibrary.PrintString` (`KismetStringLibrary.Concat_StrStr` "Angular velocity is: " (`KismetStringLibrary.Conv_RotatorToString` _returnvalue_2)) false false (struct :`R` 0.351533 :`G` 0.982251 :`B` 0.059512 :`A` 1.0) (`self.Delta Seconds`))))
    (:`then_2`
      ;[1 1 1] 角度
      (if _success_2
        (bind _output_get (set `self.Angle` (`KismetMathLibrary.MakeRotator` (* (.roll _vector) -1.0) (* (.pitch _vector) -1.0) (.yaw _vector))))
        (`KismetSystemLibrary.PrintString` (`KismetStringLibrary.Concat_StrStr` "Angle is: " (`KismetStringLibrary.Conv_RotatorToString` _output_get)) false false (struct :`R` 0.351532 :`G` 0.445201 :`B` 0.973445 :`A` 1.0) (`self.Delta Seconds`))))
    (:`then_3`
      ;[1 1 1] 座標の同期
      (`SceneComponent.K2_SetRelativeRotation` (`self.Joycon`) _angle false false)
      (`SceneComponent.K2_SetRelativeLocation` (`self.Joycon`) (* (* (`KismetMathLibrary.MakeVector` 0.0 (.yaw _angle) (.pitch _angle)) -1.0) (`self.sensitivity`)) false false))))

(fn `UserConstructionScript`)